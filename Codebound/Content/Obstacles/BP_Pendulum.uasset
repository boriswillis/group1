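; BP_Pendulum is a swinging obstacle that knocks the third-person player character away on impact.
; On BeginPlay, a timeline drives the merged component's relative rotation, interpolating pitch between the two ends of the swing arc.
; A hit on the Collision component casts the other actor to BP_ThirdPersonCharacter and launches it along the scaled hit normal impulse, with added lift along the pendulum's up vector.
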(event `self.ReceiveBeginPlay`
  (bind (_direction _movement) (`Timeline|Movement Timeline`)
    (:`Update`
      (`SceneComponent.K2_SetRelativeRotation` (`self.Merge_05C2E618`) (`KismetMathLibrary.RLerp` (struct :`Roll` -60.0) (struct :`Roll` 60.0) _movement) false false))))

(event `self.Collision.OnComponentHit`
  (params (HitComponent :type "PrimitiveComponent Object Reference") (OtherActor :type "Actor Object Reference") (OtherComp :type "PrimitiveComponent Object Reference") (NormalImpulse :type "Vector Structure") (Hit :type "HitResult Structure (by ref)"))
  (bind _asbp_third_person_character (cast `/Game/ThirdPerson/Blueprints/BP_ThirdPersonCharacter` OtherActor))
  (`Character.LaunchCharacter` _asbp_third_person_character (+ (* NormalImpulse 1500.0) (* (`self.GetActorUpVector`) 150.0)) false false))

(fn `UserConstructionScript`)